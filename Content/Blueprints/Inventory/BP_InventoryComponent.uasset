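; Inventory component that stores the owner's items as an array of item structs, with functions to add and find them.
; On BeginPlay it calls CreateInventory, which calls a still-empty LoadInventory stub.
; TryAddItem matches by ID, raising a stackable item's quantity by one, rejecting non-stackable duplicates and appending new types.
; FindItem resolves a row name through DT_Items, then searches the array for that ID.
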(event EventBeginPlay
  (CallFunction|CreateInventory))

(fn CreateInventory
  (CallFunction|LoadInventory))

(fn LoadInventory)

(fn TryAddItem
  (params (ItemToAdd :type ST%20Item%20Structure))
  (LocalVariables|SetHasItem? false)
  ;[0.15 0.15 0.15 0.5] Finding Item
  (bind (_array_element _array_index) (Utilities|Array|ForEachLoopwithBreak (Variables|Default|GetInventory) :!label _label)
    (:LoopBody
      (if (Utilities|Enum|Equal(Enum) (.ID (Utilities|Struct|BreakST_Item _array_element)) (.ID (Utilities|Struct|BreakST_Item ItemToAdd)))
        (LocalVariables|SetHasItem? true)
        (LocalVariables|SetItemInfo _array_element)
        (LocalVariables|SetItemIndex _array_index)
        (goto _label Break)))
    (:Completed
      (if (LocalVariables|GetHasItem?)
        ;[0.15 0.15 0.15 0.5] Check Stackable
        (if (.Stackable (Utilities|Struct|BreakST_Item (LocalVariables|GetItemInfo)))
          ;[0.15 0.15 0.15 0.5] Stacking Item
          (Utilities|Array|SetArrayElem (Variables|Default|GetInventory) (LocalVariables|GetItemIndex) (Utilities|Struct|MakeST_Item (.ID (Utilities|Struct|BreakST_Item (LocalVariables|GetItemInfo))) (.Name (Utilities|Struct|BreakST_Item (LocalVariables|GetItemInfo))) (.Stackable (Utilities|Struct|BreakST_Item (LocalVariables|GetItemInfo))) (+ (.Quantity (Utilities|Struct|BreakST_Item (LocalVariables|GetItemInfo))) 1) (.Icon (Utilities|Struct|BreakST_Item (LocalVariables|GetItemInfo)))) true)
          (return true)
          (else
            (Development|PrintString "HAS ITEM, AND CANT STACK")
            (return false)))
        (else
          ;[0.15 0.15 0.15 0.5] First Item Type In Inventory
          (Utilities|Array|AddUnique (Variables|Default|GetInventory) ItemToAdd)
          (Development|PrintString (Utilities|String|Append (Utilities|String|ToString(Name) (.Name (Utilities|Struct|BreakST_Item ItemToAdd))) " Added"))
          (return true))))))

(fn FindItem
  (params (RowName :type Name))
  (bind _returnvalue (Utilities|GetDataTableRow "/Game/Blueprints/Inventory/Data/DT_Items.DT_Items" RowName)
    (:then
      (bind (_array_element _array_index) (Utilities|Array|ForEachLoopwithBreak (Variables|Default|GetInventory) :!label _label)
        (:LoopBody
          (if (Utilities|Enum|Equal(Enum) (.ID (Utilities|Struct|BreakST_Item _array_element)) (.ID (Utilities|Struct|BreakST_Item _returnvalue)))
            (LocalVariables|SetHasItem? true)
            (goto _label Break)))
        (:Completed
          (return (LocalVariables|GetHasItem?) _array_element _array_index))))))