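; Seamless linked portal actor that shows the view through its LinkedPortal and teleports the player there for a loop transition.
; When Portal is set, BeginPlay feeds the linked camera's render target into the plane's material and clips its own capture.
; Each post-update tick mirrors the player camera onto the linked capture and tests for front-to-back plane crossings.
; Crossing remaps the character's transform, control rotation and velocity into the linked portal's space.
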(event EventBeginPlay
  (bind _linkedportal (Variables|Portal|GetLinkedPortal))
  (if (Variables|Default|GetPortal?)
    ;[0.15 0.15 0.15 0.5] Creating Capture
    (Components|Tick|SetTickGroup "TG_PostUpdateWork")
    (bind _returnvalue (Rendering|CreateRenderTarget2D 1920 1080 "RTF_RGBA16f"))
    (Variables|Default|SetPortal_RenderTarget _returnvalue)
    (bind _returnvalue_2 (Rendering|Material|CreateDynamicMaterialInstance (Variables|Default|GetPortalPlane) 0 "/Game/Blueprints/LoopTransition/M_Portal.M_Portal" "None" :!class /Script/Engine.PrimitiveComponent))
    (Variables|Default|SetM_Portal_Instance _returnvalue_2)
    (Utilities|IsValid _linkedportal
      (:Is%20Valid
        (bind _output_get (Variables|/Script/Engine.SceneCaptureComponent2D|SetTextureTarget (Variables|BP_LoopTransition_C|GetPortalCamera _linkedportal) (Variables|Default|GetPortal_RenderTarget)))
        (Rendering|Material|SetTextureParameterValue (Variables|Default|GetM_Portal_Instance) "texture" _output_get)
        (CallFunction|SetClipPlanes))
      (:Is%20Not%20Valid
        (Development|PrintString "Hello")))
    (else
      (Actor|Tick|SetActorTickEnabled false)
      (Rendering|ToggleVisibility (Variables|Default|GetPortalPlane) true))))

(event EventTick
  (params (DeltaSeconds :type Float%20%28single-precision%29))
  ;[0.15 0.15 0.15 0.5] TICK
  (CallFunction|UpdateSceneCapture)
  (CallFunction|ShouldTelport?))

(fn ConstructionScript)

(fn UpdateSceneCapture
  (bind _returnvalue (Transformation|GetActorTransform))
  (bind _returnvalue_2 (Transformation|GetActorTransform))
  (bind _returnvalue_3 (Game|GetPlayerCameraManager 0))
  (bind _linkedportal (Variables|Portal|GetLinkedPortal))
  (bind _linkedportal_2 (Variables|Portal|GetLinkedPortal))
  (bind _returnvalue_4 (Transformation|GetActorTransform _linkedportal_2))
  (bind (_x _y _z) (Math|Vector|BreakVector (.scale _returnvalue)))
  (bind _transformcomponent (Variables|/Script/Engine.PlayerCameraManager|GetTransformComponent _returnvalue_3))
  (bind _returnvalue_5 (Transformation|GetWorldRotation _transformcomponent))
  (bind (_x_2 _y_2 _z_2) (Math|Rotator|BreakRotIntoAxes _returnvalue_5))
  (Utilities|IsValid _linkedportal
    (:Is%20Valid
      (Transformation|SetWorldLocationAndRotation (Variables|BP_LoopTransition_C|GetPortalCamera _linkedportal) (Math|Transform|TransformLocation (Transformation|GetActorTransform (Variables|Portal|GetLinkedPortal)) (Math|Transform|InverseTransformLocation (Math|Transform|MakeTransform (.location _returnvalue) (.rotation _returnvalue) (Math|Vector|MakeVector (* _x -1.0) (* _y -1.0) _z)) (Transformation|GetWorldLocation (Variables|/Script/Engine.PlayerCameraManager|GetTransformComponent (Game|GetPlayerCameraManager 0))))) (Math|Rotator|MakeRotationfromAxes (Math|Transform|TransformDirection _returnvalue_4 (Math|Vector|MirrorVectorbyNormal (Math|Vector|MirrorVectorbyNormal (Math|Transform|InverseTransformDirection _returnvalue_2 _x_2) "1.000000,0.000000,0.000000") "0.000000,1.000000,0.000000")) (Math|Transform|TransformDirection _returnvalue_4 (Math|Vector|MirrorVectorbyNormal (Math|Vector|MirrorVectorbyNormal (Math|Transform|InverseTransformDirection _returnvalue_2 _y_2) "1.000000,0.000000,0.000000") "0.000000,1.000000,0.000000")) (Math|Transform|TransformDirection _returnvalue_4 (Math|Vector|MirrorVectorbyNormal (Math|Vector|MirrorVectorbyNormal (Math|Transform|InverseTransformDirection _returnvalue_2 _z_2) "1.000000,0.000000,0.000000") "0.000000,1.000000,0.000000"))) false false))))

(fn SetClipPlanes
  (bind _portalcamera (Variables|Default|GetPortalCamera))
  (Utilities|IsValid (Variables|Portal|GetLinkedPortal)
    (:Is%20Valid
      (Variables|/Script/Engine.SceneCaptureComponent2D|SetbEnableClipPlane _portalcamera true)
      (Variables|/Script/Engine.SceneCaptureComponent2D|SetClipPlaneBase _portalcamera (+ (Transformation|GetWorldLocation (Variables|Default|GetPortalPlane)) (* (Math|Vector|GetForwardVector (Variables|Default|GetForwardDirection)) -3.0)))
      (Variables|/Script/Engine.SceneCaptureComponent2D|SetClipPlaneNormal _portalcamera (Math|Vector|GetForwardVector (Variables|Default|GetForwardDirection))))))

(fn IsPointCrossingPortal
  (params (Point :type Vector) (PortalLocation :type Vector) (PortalNormal :type Vector))
  (LocalVariables|SetisInFront (>= (Math|Vector|DotProduct PortalNormal (- Point PortalLocation)) 0.0))
  (bind _output_get (LocalVariables|SetPortalPlane (Class|KismetMathLibrary|MakePlanefromPointandNormal PortalLocation PortalNormal)))
  (LocalVariables|SetIsIntersect (.ReturnValue (Class|KismetMathLibrary|LinePlaneIntersection (Variables|Default|GetLastPosition) Point _output_get)))
  (LocalVariables|SetisCrossing? (Math|Boolean|ANDBoolean (LocalVariables|GetIsIntersect) (not (LocalVariables|GetisInFront)) (Variables|Default|GetLastInFront)))
  (Variables|Default|SetLastInFront (LocalVariables|GetisInFront))
  (Variables|Default|SetLastPosition Point)
  (return (LocalVariables|GetisCrossing?)))

(fn ShouldTelport?
  (Utilities|IsValid (Utilities|Array|Get(acopy) (Collision|GetOverlappingActors (Variables|Default|GetPlayerDetection) "/Game/Blueprints/BP_FirstPersonCharacter.BP_FirstPersonCharacter_C" :!class /Script/Engine.PrimitiveComponent))
    (:Is%20Valid
      (bind _return (CallFunction|IsPointCrossingPortal (Transformation|GetWorldLocation (Variables|/Game/Blueprints/BP_FirstPersonCharacter.BP_FirstPersonCharacter_C|GetFirstPersonCamera (.AsBP%20First%20Person%20Character (Utilities|Casting|CastToBP_FirstPersonCharacter (Game|GetPlayerCharacter 0))))) (Transformation|GetActorLocation) (Math|Vector|GetForwardVector (Variables|Default|GetForwardDirection))))
      (if _return
        (CallFunction|TeleportCharacter)))))

(fn TeleportCharacter
  (bind _returnvalue (Transformation|GetActorTransform))
  (bind _returnvalue_2 (Transformation|GetActorTransform))
  (bind _returnvalue_3 (Transformation|GetActorTransform))
  (bind _returnvalue_4 (Game|GetPlayerCharacter 0))
  (bind _returnvalue_5 (Game|GetPlayerController 0))
  (bind _returnvalue_6 (Game|GetPlayerCharacter 0))
  (bind _linkedportal (Variables|Portal|GetLinkedPortal))
  (bind _linkedportal_2 (Variables|Portal|GetLinkedPortal))
  (bind _returnvalue_7 (Transformation|GetActorTransform _linkedportal))
  (bind (_x _y _z) (Math|Vector|BreakVector (.scale _returnvalue)))
  (bind _returnvalue_8 (Transformation|GetActorRotation _returnvalue_4))
  (bind _returnvalue_9 (Transformation|GetActorTransform _linkedportal_2))
  (bind _returnvalue_10 (Pawn|GetControlRotation _returnvalue_5 :!class /Script/Engine.Controller))
  (bind _charactermovement (Variables|/Script/Engine.Character|GetCharacterMovement _returnvalue_6))
  (bind (_x_2 _y_2 _z_2) (Math|Rotator|GetAxes _returnvalue_10))
  (bind (_x_3 _y_3 _z_3) (Math|Rotator|GetAxes _returnvalue_8))
  (Transformation|SetActorTransform (Game|GetPlayerCharacter 0) (Math|Transform|MakeTransform (Math|Transform|TransformLocation (Transformation|GetActorTransform (Variables|Portal|GetLinkedPortal)) (Math|Transform|InverseTransformLocation (Math|Transform|MakeTransform (.location _returnvalue) (.rotation _returnvalue) (Math|Vector|MakeVector (* _x -1.0) (* _y -1.0) _z)) (Transformation|GetActorLocation (Game|GetPlayerCharacter 0)))) (Math|Rotator|MakeRotationfromAxes (Math|Transform|TransformDirection _returnvalue_9 (Math|Vector|MirrorVectorbyNormal (Math|Vector|MirrorVectorbyNormal (Math|Transform|InverseTransformDirection _returnvalue_3 _x_3) "1.000000,0.000000,0.000000") "0.000000,1.000000,0.000000")) (Math|Transform|TransformDirection _returnvalue_9 (Math|Vector|MirrorVectorbyNormal (Math|Vector|MirrorVectorbyNormal (Math|Transform|InverseTransformDirection _returnvalue_3 _y_3) "1.000000,0.000000,0.000000") "0.000000,1.000000,0.000000")) (Math|Transform|TransformDirection _returnvalue_9 (Math|Vector|MirrorVectorbyNormal (Math|Vector|MirrorVectorbyNormal (Math|Transform|InverseTransformDirection _returnvalue_3 _z_3) "1.000000,0.000000,0.000000") "0.000000,1.000000,0.000000"))) "1.000000,1.000000,1.000000"))
  (Pawn|SetControlRotation (Game|GetPlayerController 0) (Math|Rotator|MakeRotationfromAxes (Math|Transform|TransformDirection _returnvalue_7 (Math|Vector|MirrorVectorbyNormal (Math|Vector|MirrorVectorbyNormal (Math|Transform|InverseTransformDirection _returnvalue_2 _x_2) "1.000000,0.000000,0.000000") "0.000000,1.000000,0.000000")) (Math|Transform|TransformDirection _returnvalue_7 (Math|Vector|MirrorVectorbyNormal (Math|Vector|MirrorVectorbyNormal (Math|Transform|InverseTransformDirection _returnvalue_2 _y_2) "1.000000,0.000000,0.000000") "0.000000,1.000000,0.000000")) (Math|Transform|TransformDirection _returnvalue_7 (Math|Vector|MirrorVectorbyNormal (Math|Vector|MirrorVectorbyNormal (Math|Transform|InverseTransformDirection _returnvalue_2 _z_2) "1.000000,0.000000,0.000000") "0.000000,1.000000,0.000000"))))
  (bind _returnvalue_11 (CallFunction|UpdateVelocity (Variables|/Script/Engine.MovementComponent|GetVelocity _charactermovement)))
  (Variables|/Script/Engine.MovementComponent|SetVelocity _charactermovement _returnvalue_11))

(fn UpdateVelocity
  (params (Velocity :type Vector))
  (return (* (Math|Transform|TransformDirection (Transformation|GetActorTransform (Variables|Portal|GetLinkedPortal)) (Math|Vector|MirrorVectorbyNormal (Math|Vector|MirrorVectorbyNormal (Math|Transform|InverseTransformDirection (Transformation|GetActorTransform) (Math|Vector|Normalize Velocity)) "1.000000,0.000000,0.000000") "0.000000,1.000000,0.000000")) (Math|Vector|VectorLength Velocity))))