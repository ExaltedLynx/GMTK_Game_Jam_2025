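; Replicator gun that copies a puzzle object and places a clone of it.
; Copying spawns a BP_ReplicatorCopiedObject preview from the source's mesh and transform and calls a grab on the player's physics handle at its location.
; Placing spawns a new actor of the source's class at the preview's transform, registers it through ClonedObjectRefs, destroys the preview and clears the copy state.
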(event EventBeginPlay)

(event EventTick
  (params (DeltaSeconds :type Float%20%28single-precision%29)))

(fn CopyPuzzleObject
  (params (HitActor :type Puzzle%20Object%20Object%20Reference))
  (bind _output_get (Variables|Default|SetCopiedObject HitActor))
  (bind _returnvalue (Game|SpawnActorfromClass "/Game/Blueprints/Replicator/BP_ReplicatorCopiedObject.BP_ReplicatorCopiedObject_C" (Transformation|GetActorTransform HitActor) "Undefined" "MultiplyWithRoot" 0 0))
  (Default|InitCopiedObject _returnvalue (Default|GetObjectMesh _output_get))
  (Class|PhysicsHandleComponent|GrabComponentatLocation (Variables|/Game/Blueprints/Player/BP_FirstPersonCharacter.BP_FirstPersonCharacter_C|GetPhysicsHandle (Variables|Default|GetPlayer)) 0 "None" (Transformation|GetActorLocation _returnvalue))
  (Variables|Default|SetObjPreviewInst _returnvalue)
  (Variables|Default|SetHasCopiedObject? true))

(fn SpawnCopiedObjectClone
  (Utilities|FlowControl|Sequence
    (:then_0
      (bind _returnvalue (Game|SpawnActorfromClass (Utilities|GetClass (Variables|Default|GetCopiedObject)) (Transformation|GetActorTransform (Variables|Default|GetObjPreviewInst)) "Undefined" "MultiplyWithRoot" 0 0))
      (Default|SetClone (Variables|Default|GetClonedObjectRefs) _returnvalue)
      (Actor|DestroyActor (Variables|Default|GetObjPreviewInst)))
    (:then_1
      (Variables|Default|SetHasCopiedObject? false)
      (Variables|Default|SetCopiedObject 0)
      (Variables|Default|SetObjPreviewInst 0))))

(fn GetHasCopiedObject
  (return (Variables|Default|GetHasCopiedObject?)))