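; BP_ClonedObjectsRefs is a level registry that tracks the current replicator clone for each puzzle object type, so only one clone per type exists.
; On BeginPlay it registers itself with the player character's ReplicatorGun component.
; SetClone destroys any existing clone of the same type before storing the new one, with GetClone and DeleteClone switching on the type enum.
; Only the Cube type is currently handled.
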(event EventBeginPlay
  (Variables|/Game/Blueprints/Replicator/ReplicatorGun.ReplicatorGun_C|SetClonedObjectRefs (Actor|GetComponentbyClass (Game|GetPlayerCharacter 0) "/Game/Blueprints/Replicator/ReplicatorGun.ReplicatorGun_C") self))

(event Collision|EventActorBeginOverlap
  (params (OtherActor :type Actor%20Object%20Reference)))

(event EventTick
  (params (DeltaSeconds :type Float%20%28single-precision%29)))

(fn ConstructionScript)

(fn DeleteClone
  (params (CloneObjectType :type PuzzleObjectTypes%20Enum :default "NewEnumerator0"))
  (switch Utilities|FlowControl|Switch|SwitchonPuzzleObjectTypes CloneObjectType
    (:NewEnumerator0
      (Actor|DestroyActor (Variables|Default|GetCubeClone)))))

(fn SetClone
  (params (ClonedObject :type Puzzle%20Object%20Object%20Reference))
  (bind _objecttype (Variables|/Game/Blueprints/Interactables/PuzzleObjects/PuzzleObject.PuzzleObject_C|GetObjectType ClonedObject))
  (bind _clonedobject (CallFunction|GetClone _objecttype))
  (if (Utilities|IsValid _clonedobject)
    (CallFunction|DeleteClone _objecttype))
  (switch Utilities|FlowControl|Switch|SwitchonPuzzleObjectTypes _objecttype
    (:NewEnumerator0
      (Variables|Default|SetCubeClone ClonedObject))))

(fn GetClone
  (params (PuzzleObjectType :type PuzzleObjectTypes%20Enum :default "NewEnumerator0"))
  (switch Utilities|FlowControl|Switch|SwitchonPuzzleObjectTypes PuzzleObjectType
    (:NewEnumerator0
      (bind _output_get (LocalVariables|SetcloneOfType (Variables|Default|GetCubeClone)))
      (return _output_get))))