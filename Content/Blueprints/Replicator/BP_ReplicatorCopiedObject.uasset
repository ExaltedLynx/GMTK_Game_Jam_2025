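; BP_ReplicatorCopiedObject is the preview actor for an object copied by the replicator, held by a player.
; InitCopiedObject stores the grabbing player, applies the given mesh with a preview material on its first slot and enables physics simulation.
; Each tick moves the player's PhysicsHandle target to their interact location.
; Actor overlap events toggle CanBePlaced without counting overlaps, so any end overlap marks it placeable.
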(event EventBeginPlay)

(event Collision|EventActorBeginOverlap
  (params (OtherActor :type Actor%20Object%20Reference))
  (Variables|Default|SetCanBePlaced? false))

(event EventTick
  (params (DeltaSeconds :type Float%20%28single-precision%29))
  (bind _grabbingplayer (Variables|Default|GetGrabbingPlayer))
  (Physics|Components|PhysicsHandle|SetTargetLocation (Variables|/Game/Blueprints/Player/BP_FirstPersonCharacter.BP_FirstPersonCharacter_C|GetPhysicsHandle _grabbingplayer) (Default|GetInteractLocation _grabbingplayer)))

(event Collision|EventActorEndOverlap
  (params (OtherActor :type Actor%20Object%20Reference))
  (Variables|Default|SetCanBePlaced? true))

(fn ConstructionScript)

(fn InitCopiedObject
  (params (ObjectMesh :type Static%20Mesh%20Object%20Reference) (GrabbingPlayer :type BP%20First%20Person%20Character%20Object%20Reference))
  (bind _copiedobjmesh (Variables|Default|GetCopiedObjMesh))
  (Variables|Default|SetGrabbingPlayer GrabbingPlayer)
  (Components|StaticMesh|SetStaticMesh _copiedobjmesh ObjectMesh)
  (Rendering|Material|SetMaterial _copiedobjmesh 0 "/Game/Materials/ObjectPreviewMat.ObjectPreviewMat")
  (Physics|SetSimulatePhysics _copiedobjmesh true))