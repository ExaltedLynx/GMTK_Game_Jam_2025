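; BP_RespawnManager spawns a first-person player character at its SpawnPoint transform and has player controller 0 possess it.
; It spawns on BeginPlay when Active is set, and RespawnPlayer reruns the same path without that check, ignoring its InPawn argument.
; Before possession, ResetCharacterValues sets capsule collision to QueryAndProbe, restores walking movement and makes the sprite visible.
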(event Custom|RespawnPlayer
  (params (InPawn :type Pawn%20Object%20Reference))
  (bind _spawnpoint (Variables|Default|GetSpawnPoint))
  (bind _returnvalue (Transformation|GetWorldTransform _spawnpoint))
  (bind _returnvalue_2 (Game|SpawnActorfromClass "/Game/Blueprints/Player/BP_FirstPersonCharacter.BP_FirstPersonCharacter_C" (Math|Transform|MakeTransform (.location _returnvalue) (.rotation _returnvalue) "1.000000,1.000000,1.000000") "Undefined" "MultiplyWithRoot" 0 0))
  (CallFunction|ResetCharacterValues _returnvalue_2)
  (Pawn|Possess (Game|GetPlayerController 0) _returnvalue_2))

(event EventBeginPlay
  (bind _spawnpoint (Variables|Default|GetSpawnPoint))
  (bind _returnvalue (Transformation|GetWorldTransform _spawnpoint))
  (if (Variables|Default|GetActive?)
    (bind _returnvalue_2 (Game|SpawnActorfromClass "/Game/Blueprints/Player/BP_FirstPersonCharacter.BP_FirstPersonCharacter_C" (Math|Transform|MakeTransform (.location _returnvalue) (.rotation _returnvalue) "1.000000,1.000000,1.000000") "Undefined" "MultiplyWithRoot" 0 0))
    (CallFunction|ResetCharacterValues _returnvalue_2)
    (Pawn|Possess (Game|GetPlayerController 0) _returnvalue_2)))

(fn ConstructionScript)

(fn ResetCharacterValues
  (params (Character :type BP%20First%20Person%20Character%20Object%20Reference))
  (Collision|SetCollisionEnabled (Variables|/Script/Engine.Character|GetCapsuleComponent Character) "QueryAndProbe")
  (Pawn|Components|CharacterMovement|SetMovementMode (Variables|/Script/Engine.Character|GetCharacterMovement Character) "MOVE_Walking" 0)
  (Rendering|SetVisibility (Variables|/Script/Paper2D.PaperCharacter|GetSprite Character) true false))