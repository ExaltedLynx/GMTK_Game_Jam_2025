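; Base HUD class that creates and owns the main HUD widget and the pause menu widget.
; On BeginPlay, a shared helper instantiates both from template classes for the owning player and adds them to the viewport.
; Show and hide pause menu events toggle that menu's visibility, mouse cursor and UI-only or game-only input mode on player controller 0.
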(event EventBeginPlay
  (CallFunction|CreateWidgets))

(event EventHidePauseMenu
  (bind _returnvalue (Game|GetPlayerController 0))
  (Widget|SetVisibility (Variables|Default|GetPauseMenuWidget) "Collapsed")
  (Variables|/Script/Engine.PlayerController|SetbShowMouseCursor _returnvalue false)
  (Input|SetInputModeGameOnly _returnvalue true))

(event EventShowPauseMenu
  (bind _returnvalue (Game|GetPlayerController 0))
  (Widget|SetVisibility (Variables|Default|GetPauseMenuWidget) "Visible")
  (Variables|/Script/Engine.PlayerController|SetbShowMouseCursor _returnvalue true)
  (Input|SetInputModeUIOnly _returnvalue 0 "DoNotLock" true))

(fn ConstructionScript)

(fn AddNewWidget
  (params (WidgetTemplate :type User%20Widget%20Class%20Reference) (AddToViewport :type Boolean))
  (bind _widgettemplate (LocalVariables|GetWidgetTemplate)
    (:then
      (bind _returnvalue (UserInterface|CreateWidget _widgettemplate (Game|Player|GetOwningPlayerController)))
      (LocalVariables|SetNew%20Widget%20Instance _returnvalue)
      (Utilities|FlowControl|Sequence
        (:then_0
          (if AddToViewport
            (UserInterface|Viewport|AddtoViewport (LocalVariables|GetNew%20Widget%20Instance) 0)))
        (:then_1
          (return (LocalVariables|GetNew%20Widget%20Instance)))))
    (:else)))

(fn CreateWidgets
  (bind _spawned_widget (CallFunction|AddNewWidget (Variables|Default|GetHUD%20Widget%20Template) true))
  (Variables|Default|SetHUD%20Widget _spawned_widget)
  (bind _spawned_widget_2 (CallFunction|AddNewWidget (Variables|Default|GetPause%20Menu%20Template) true))
  (Variables|Default|SetPauseMenuWidget _spawned_widget_2))