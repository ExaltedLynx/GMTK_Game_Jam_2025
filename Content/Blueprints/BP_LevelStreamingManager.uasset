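; Level streaming trigger actor that swaps sublevels when BP_FirstPersonCharacter overlaps its TransitionA component.
; It unloads every name in LevelsToUnload, then loads and shows every name in LevelsToLoad, using non-blocking latent calls chained through a shared LevelIndex.
; An empty unload list only prints a warning and skips loading.
; The DoOnce node is disconnected, so nothing guards against repeat overlaps.
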(event OnComponentBeginOverlap(TransitionA)
  (params (OverlappedComponent :type Primitive%20Component%20Object%20Reference) (OtherActor :type Actor%20Object%20Reference) (OtherComp :type Primitive%20Component%20Object%20Reference) (OtherBodyIndex :type Integer) (bFromSweep :type Boolean) (SweepResult :type Hit%20Result%20Structure%20%28by%20ref%29))
  ;[0.15 0.15 0.15 0.5] LevelStreaming
  (Utilities|Casting|CastToBP_FirstPersonCharacter OtherActor)
  (if (== (Utilities|Array|Length (Variables|Default|GetLevelsToUnload)) 0)
    (Development|PrintString "NO LEVELS ASSIGN")
    (else
      (Game|UnloadStreamLevel(byName) (Utilities|Array|Get(acopy) (Variables|Default|GetLevelsToUnload) (Variables|Default|GetLevelIndex)) false :!label _label)
      (Math|Integer|IncrementInt (Variables|Default|GetLevelIndex)
        (:%20%20
          (if (>= (Variables|Default|GetLevelIndex) (Utilities|Array|Length (Variables|Default|GetLevelsToUnload)))
            (Variables|Default|SetLevelIndex 0)
            (Game|LoadStreamLevel(byName) (Utilities|Array|Get(acopy) (Variables|Default|GetLevelsToLoad) (Variables|Default|GetLevelIndex)) true :!label _label_2)
            (Math|Integer|IncrementInt (Variables|Default|GetLevelIndex)
              (:%20%20
                (if (>= (Variables|Default|GetLevelIndex) (Utilities|Array|Length (Variables|Default|GetLevelsToLoad)))
                  (Variables|Default|SetLevelIndex 0)
                  (else
                    (goto _label_2)))))
            (else
              (goto _label))))))))

(event EventBeginPlay)

(event Collision|EventActorBeginOverlap
  (params (OtherActor :type Actor%20Object%20Reference)))

(event EventTick
  (params (DeltaSeconds :type Float%20%28single-precision%29)))

(fn ConstructionScript)