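; BP_PuzzleObject_Vent is an interactable vent puzzle object that stays fixed until a player grabs it.
; BeginPlay sets the PuzzleCube component to WorldDynamic with physics off.
; HandleInteract switches it to a simulating PhysicsBody, grabs the hit component with the interactor's PhysicsHandle, and records the held state and grabbing player.
; This Blueprint contains no release logic and never turns physics back off after the grab.
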(event EventBeginPlay
  (|CallParentFunction)
  (Collision|SetCollisionObjectType (Variables|Default|GetPuzzleCube) "ECC_WorldDynamic")
  (Physics|SetSimulatePhysics (Variables|Default|GetPuzzleCube) false))

(event Collision|EventActorBeginOverlap
  (params (OtherActor :type Actor%20Object%20Reference))
  (|CallParentFunction OtherActor) ; This node is disabled and will not be called.\nDrag off pins to build functionality.
)

(event EventTick
  (params (DeltaSeconds :type Float%20%28single-precision%29))
  (|CallParentFunction DeltaSeconds) ; This node is disabled and will not be called.\nDrag off pins to build functionality.
)

(event EventHandleInteract
  (params (Interactor :type BP%20First%20Person%20Character%20Object%20Reference) (PrimitiveComp :type Primitive%20Component%20Object%20Reference) (LocationHit :type Vector :default "0, 0, 0"))
  (bind _puzzlecube (Variables|Default|GetPuzzleCube))
  (Collision|SetCollisionObjectType _puzzlecube "ECC_PhysicsBody")
  (Physics|SetSimulatePhysics _puzzlecube true)
  (Physics|Components|PhysicsHandle|GrabComponentatLocationwithRotation (Variables|/Game/Blueprints/Player/BP_FirstPersonCharacter.BP_FirstPersonCharacter_C|GetPhysicsHandle Interactor) PrimitiveComp "None" LocationHit "0, 0, 0")
  (Variables|/Game/Blueprints/Player/BP_FirstPersonCharacter.BP_FirstPersonCharacter_C|SetisHoldingObject? Interactor true)
  (Variables|Default|SetIsGrabbed? true)
  (Variables|Default|SetGrabbingPlayer Interactor))

(fn ConstructionScript
  (|CallParentFunction))