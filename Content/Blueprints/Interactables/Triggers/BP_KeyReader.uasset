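; BP_KeyReader is an interactable trigger that works only when the player's inventory holds a required item.
; On interact, it looks up ItemToFind in the BP_InventoryComponent of player character 0.
; If found, it turns the Read component's surface color green and calls the parent interact handler, gated by a DoOnce so this happens a single time.
; Otherwise, it only prints a message naming the missing item.
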(event EventBeginPlay
  (|CallParentFunction) ; This node is disabled and will not be called.\nDrag off pins to build functionality.
)

(event Collision|EventActorBeginOverlap
  (params (OtherActor :type Actor%20Object%20Reference))
  (|CallParentFunction OtherActor) ; This node is disabled and will not be called.\nDrag off pins to build functionality.
)

(event EventTick
  (params (DeltaSeconds :type Float%20%28single-precision%29))
  (|CallParentFunction DeltaSeconds) ; This node is disabled and will not be called.\nDrag off pins to build functionality.
)

(event EventHandleInteract
  (params (Interactor :type BP%20First%20Person%20Character%20Object%20Reference) (PrimitiveComp :type Primitive%20Component%20Object%20Reference) (InteractedActor :type Actor%20Object%20Reference) (LocationHit :type Vector :default "0, 0, 0"))
  (bind _hasitem__ (Default|FindItem (Actor|GetComponentbyClass (Game|GetPlayerCharacter 0) "/Game/Blueprints/Inventory/BP_InventoryComponent.BP_InventoryComponent_C") (Variables|Default|GetItemToFind)))
  (if _hasitem__
    (Utilities|FlowControl|DoOnce false
      (:Completed
        (Rendering|Material|SetColorParameterValueonMaterials (Variables|Default|GetRead) "SurfaceColor" "(R=0.242774,G=1.000000,B=0.138531,A=1.000000)")
        (|CallParentFunction Interactor PrimitiveComp InteractedActor LocationHit)))
    (else
      (Development|PrintString (Utilities|String|Append "Does not have " (Utilities|String|ToString(Name) (Variables|Default|GetItemToFind)))))))

(fn ConstructionScript
  (|CallParentFunction))