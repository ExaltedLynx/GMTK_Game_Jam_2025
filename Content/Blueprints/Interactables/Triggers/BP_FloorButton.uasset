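; A floor button interactable that activates when something overlaps its trigger and again when the overlap ends.
; On BeginPlay it fetches the symbol actor from its ButtonTriggerSymbol child actor component and sets its letter from TriggerSymbol.
; Overlap begin and end switch that symbol's emission light on and off, print a debug string, then both call the same Activate.
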(event OnComponentBeginOverlap(Trigger)
  (params (OverlappedComponent :type Primitive%20Component%20Object%20Reference) (OtherActor :type Actor%20Object%20Reference) (OtherComp :type Primitive%20Component%20Object%20Reference) (OtherBodyIndex :type Integer) (bFromSweep :type Boolean) (SweepResult :type Hit%20Result%20Structure%20%28by%20ref%29))
  (Development|PrintString "on")
  (Default|ToggleEmissionLight (Variables|Default|GetTriggerSymbolLightActor) true)
  (CallFunction|Activate))

(event OnComponentEndOverlap(Trigger)
  (params (OverlappedComponent :type Primitive%20Component%20Object%20Reference) (OtherActor :type Actor%20Object%20Reference) (OtherComp :type Primitive%20Component%20Object%20Reference) (OtherBodyIndex :type Integer))
  (Development|PrintString "off")
  (Default|ToggleEmissionLight (Variables|Default|GetTriggerSymbolLightActor) false)
  (CallFunction|Activate))

(event EventBeginPlay
  (|CallParentFunction)
  (bind _output_get (Variables|Default|SetTriggerSymbolLightActor (CallFunction|GetTriggerSymbolLightActor)))
  (Default|SetSymbolText _output_get (CallFunction|GetTriggerSymbolLetter (Variables|Default|GetTriggerSymbol))))

(event EventTick
  (params (DeltaSeconds :type Float%20%28single-precision%29))
  (|CallParentFunction DeltaSeconds) ; This node is disabled and will not be called.\nDrag off pins to build functionality.
)

(fn ConstructionScript
  (|CallParentFunction))

(fn GetTriggerSymbolLightActor
  (bind _asbutton_trigger_symbol (Utilities|Casting|CastToButtonTriggerSymbol (Variables|/Script/Engine.ChildActorComponent|GetChildActor (Variables|Default|GetButtonTriggerSymbol))))
  (return _asbutton_trigger_symbol))