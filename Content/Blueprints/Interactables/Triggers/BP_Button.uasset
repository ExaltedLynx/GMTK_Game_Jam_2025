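; BP_Button is an interactable button trigger that shows its trigger symbol and on/off state.
; On BeginPlay it fetches its ButtonTriggerSymbol child actor and sets that actor's text to the letter for its TriggerSymbol.
; Activate runs the parent logic, then uses Active to color the Cylinder green or red and switch the symbol's emission light on or off.
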(event EventBeginPlay
  (|CallParentFunction)
  (bind _output_get (Variables|Default|SetTriggerSymbolLightActor (CallFunction|GetTriggerSymbolLightActor)))
  (Default|SetSymbolText _output_get (CallFunction|GetTriggerSymbolLetter (Variables|Default|GetTriggerSymbol))))

(event Collision|EventActorBeginOverlap
  (params (OtherActor :type Actor%20Object%20Reference))
  (|CallParentFunction OtherActor) ; This node is disabled and will not be called.\nDrag off pins to build functionality.
)

(event EventTick
  (params (DeltaSeconds :type Float%20%28single-precision%29))
  (|CallParentFunction DeltaSeconds) ; This node is disabled and will not be called.\nDrag off pins to build functionality.
)

(event EventActivate
  (bind _triggersymbollightactor (Variables|Default|GetTriggerSymbolLightActor))
  (|CallParentFunction)
  (if (Variables|Default|GetActive?)
    (Rendering|Material|SetColorParameterValueonMaterials (Variables|Default|GetCylinder) "SurfaceColor" "(R=0.238724,G=1.000000,B=0.000954,A=1.000000)")
    (Default|ToggleEmissionLight _triggersymbollightactor true)
    (else
      (Rendering|Material|SetColorParameterValueonMaterials (Variables|Default|GetCylinder) "SurfaceColor" "(R=1.000000,G=0.020030,B=0.000000,A=1.000000)")
      (Default|ToggleEmissionLight _triggersymbollightactor false))))

(fn ConstructionScript
  (|CallParentFunction))

(fn GetTriggerSymbolLightActor
  (bind _asbutton_trigger_symbol (Utilities|Casting|CastToButtonTriggerSymbol (Variables|/Script/Engine.ChildActorComponent|GetChildActor (Variables|Default|GetButtonTriggerSymbol))))
  (return _asbutton_trigger_symbol))