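; BP_Trigger is an interactable trigger that activates other actors linked to it.
; HandleInteract first calls Activate to flip its Active flag, then calls TryToActivate on every entry in ActorsToTrigger, whichever state the flag ends in.
; An empty ActorsToTrigger list prints a "NO TRIGGERABLE ADDED" warning instead.
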(event Custom|Activate
  (if (Variables|Default|GetActive?)
    (Variables|Default|SetActive? false)
    (else
      (Variables|Default|SetActive? true))))

(event EventBeginPlay)

(event Collision|EventActorBeginOverlap
  (params (OtherActor :type Actor%20Object%20Reference)))

(event EventTick
  (params (DeltaSeconds :type Float%20%28single-precision%29)))

(event EventHandleInteract
  (params (Interactor :type BP%20First%20Person%20Character%20Object%20Reference) (PrimitiveComp :type Primitive%20Component%20Object%20Reference) (LocationHit :type Vector :default "0, 0, 0"))
  (bind _actorstotrigger (Variables|Default|GetActorsToTrigger))
  (CallFunction|Activate)
  (if (== (Utilities|Array|Length _actorstotrigger) 0)
    (Development|PrintString "NO TRIGGERABLE ADDED")
    (else
      (for _array_element _actorstotrigger
        (Default|TrytoActivate _array_element)))))

(fn ConstructionScript)