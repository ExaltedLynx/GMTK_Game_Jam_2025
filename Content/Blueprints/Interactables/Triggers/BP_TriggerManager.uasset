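; BP_TriggerManager assigns a symbol to every BP_Trigger in the level and shares it with the actors each one triggers.
; Shortly after BeginPlay it gathers all triggers and casts each array index to a TriggerSymbols enum value, so symbols follow the order the search returns.
; Each trigger stores its symbol, prints it for debugging, and every entry in its ActorsToTrigger receives it with the index through AddTriggerSymbol.
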(event EventBeginPlay
  (Utilities|FlowControl|Delay 0.2)
  (bind _outactors (Actor|GetAllActorsOfClass "/Game/Blueprints/Interactables/Triggers/BP_Trigger.BP_Trigger_C"))
  (CallFunction|InitTriggerSymbols _outactors))

(event Collision|EventActorBeginOverlap
  (params (OtherActor :type Actor%20Object%20Reference)))

(event EventTick
  (params (DeltaSeconds :type Float%20%28single-precision%29)))

(fn ConstructionScript)

(fn InitTriggerSymbols
  (params (Triggers :type Array%20of%20BP%20Trigger%20Object%20References))
  (for (_array_element _array_index) Triggers
    (Utilities|FlowControl|Sequence
      (:then_0
        (Development|PrintText (Utilities|Text|FormatText "{0} : {1}" (Utilities|GetDisplayName _array_element) (Utilities|String|EnumtoString (Utilities|Enum|ByteToEnumTriggerSymbols (Math|Conversions|ToByte(Integer) _array_index)))))
        (Variables|/Game/Blueprints/Interactables/Triggers/BP_Trigger.BP_Trigger_C|SetTriggerSymbol _array_element (Utilities|Enum|ByteToEnumTriggerSymbols (Math|Conversions|ToByte(Integer) _array_index))))
      (:then_1
        (for _array_element_2 (Variables|/Game/Blueprints/Interactables/Triggers/BP_Trigger.BP_Trigger_C|GetActorsToTrigger _array_element)
          (Default|AddTriggerSymbol _array_element_2 (Utilities|Enum|ByteToEnumTriggerSymbols (Math|Conversions|ToByte(Integer) _array_index)) _array_index))))))