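; Interactable hinged door that swings 90 degrees on its pivot when used and closes itself after a short delay.
; The construction script caches start and target rotations, and interaction toggles a timeline that plays or reverses the lerp between them.
; Finishing open starts a timer for self-closing, which uses a separate timeline and is cancelled by manual closing.
; Door collision switches to query-only during movement and query-and-probe afterwards.
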(event Custom|CloseDoor
  (Variables|Default|SetOpen? false)
  (Collision|SetCollisionEnabled (Variables|Default|GetDoor) "QueryOnly")
  (bind _open_close (Timeline|SelfClose PlayFromStart)
    (:Update
      (Transformation|SetRelativeRotation (Variables|Default|GetDoorPivot) (Math|Rotator|Lerp(Rotator) (Variables|Default|GetDesiredRotation) (Variables|Default|GetStartRotation) _open_close) false false))
    (:Finished
      (Collision|SetCollisionEnabled (Variables|Default|GetDoor) "QueryAndProbe")
      (Utilities|Time|ClearandInvalidateTimerbyHandle (Variables|Default|GetCloseTimer)))))

(event EventHandleInteract
  (params (Interactor :type BP%20First%20Person%20Character%20Object%20Reference) (PrimitiveComp :type Primitive%20Component%20Object%20Reference) (LocationHit :type Vector :default "0, 0, 0"))
  (Collision|SetCollisionEnabled (Variables|Default|GetDoor) "QueryOnly")
  (if (Variables|Default|GetOpen?)
    (Utilities|Time|ClearandInvalidateTimerbyHandle (Variables|Default|GetCloseTimer))
    (Variables|Default|SetOpen? false)
    (bind _open_close (Timeline|Timeline Reverse)
      (:Update
        (Transformation|SetRelativeRotation (Variables|Default|GetDoorPivot) (Math|Rotator|Lerp(Rotator) (Variables|Default|GetStartRotation) (Variables|Default|GetDesiredRotation) _open_close) false false))
      (:Finished
        (Collision|SetCollisionEnabled (Variables|Default|GetDoor) "QueryAndProbe")
        (if (Variables|Default|GetOpen?)
          (bind _returnvalue (Utilities|Time|SetTimerbyEvent (EventDispatchers|CreateEvent :!event Custom|CloseDoor) 3.0))
          (Variables|Default|SetCloseTimer _returnvalue))))
    (else
      (Variables|Default|SetOpen? true)
      (Timeline|Timeline PlayFromStart))))

(fn ConstructionScript
  (|CallParentFunction)
  (bind _output_get (Variables|Default|SetStartRotation (Variables|/Script/Engine.SceneComponent|GetRelativeRotation (Variables|Default|GetDoorPivot))))
  (Variables|Default|SetDesiredRotation (Math|Rotator|MakeRotator (.roll _output_get) (.pitch _output_get) (+ (.yaw _output_get) -9e+01))))