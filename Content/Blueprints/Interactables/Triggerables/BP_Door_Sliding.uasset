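; Sliding door interactable that toggles open and closed on interaction, or only prints a notice when it needs a trigger.
; TrytoActivate loops over the linked Triggers, stopping at the first inactive one, and sets Activate when the last is reached active.
; Both paths drive the OpenDoor timeline, which lerps the door mesh along local Y from its starting position and flips IsActive on finish.
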(event Custom|OpenClose
  ;[0.15 0.15 0.15 0.5] Open Close Animation
  (if (Variables|Default|GetisActive?)
    (bind _alpha (Timeline|OpenDoor Reverse)
      (:Update
        (Transformation|SetRelativeLocation (Variables|Default|GetDoor) (Math|Vector|Lerp(Vector) (Variables|Default|GetInitialRelativeLocation) (Variables|Default|GetDesiredRelativeLocation) _alpha) false false))
      (:Finished
        (if (Variables|Default|GetisActive?)
          (Variables|Default|SetisActive? false)
          (else
            (Variables|Default|SetisActive? true)))))
    (else
      (Timeline|OpenDoor Play))))

(event Custom|CloseDoor
  ;[0.15 0.15 0.15 0.5] Open Close Animation
  (bind _alpha (Timeline|OpenDoor ReverseFromEnd)
    (:Update
      (Transformation|SetRelativeLocation (Variables|Default|GetDoor) (Math|Vector|Lerp(Vector) (Variables|Default|GetInitialRelativeLocation) (Variables|Default|GetDesiredRelativeLocation) _alpha) false false))
    (:Finished
      (if (Variables|Default|GetisActive?)
        (Variables|Default|SetisActive? false)
        (else
          (Variables|Default|SetisActive? true))))))

(event EventBeginPlay
  (bind _door (Variables|Default|GetDoor))
  (bind _relativelocation (Variables|/Script/Engine.SceneComponent|GetRelativeLocation _door))
  (Variables|Default|SetInitialRelativeLocation _relativelocation)
  (Variables|Default|SetDesiredRelativeLocation (+ _relativelocation "0.000000,-215.000000,0.000000")))

(event EventTrytoActivate
  (bind _triggers (Variables|Default|GetTriggers))
  ;[0.15 0.15 0.15 0.5] Open Close Animation
  (bind (_array_element _array_index) (Utilities|Array|ForEachLoopwithBreak _triggers :!label _label)
    (:LoopBody
      (if (Variables|/Game/Blueprints/Interactables/Triggers/BP_Trigger.BP_Trigger_C|GetActive? _array_element)
        (if (== _array_index (- (Utilities|Array|Length _triggers) 1))
          (Variables|Default|SetActivate? true)
          (else
            (Variables|Default|SetActivate? false)))
        (else
          (goto _label Break))))
    (:Completed
      (if (Variables|Default|GetActivate?)
        (if (Variables|Default|GetisActive?)
          (bind _alpha (Timeline|OpenDoor Reverse)
            (:Update
              (Transformation|SetRelativeLocation (Variables|Default|GetDoor) (Math|Vector|Lerp(Vector) (Variables|Default|GetInitialRelativeLocation) (Variables|Default|GetDesiredRelativeLocation) _alpha) false false))
            (:Finished
              (if (Variables|Default|GetisActive?)
                (Variables|Default|SetisActive? false)
                (else
                  (Variables|Default|SetisActive? true)))))
          (else
            (Timeline|OpenDoor Play)))
        (else
          (Development|PrintString "Cant ACTIVATE"))))))

(event EventHandleInteract
  (params (Interactor :type BP%20First%20Person%20Character%20Object%20Reference) (PrimitiveComp :type Primitive%20Component%20Object%20Reference) (InteractedActor :type Actor%20Object%20Reference) (LocationHit :type Vector :default "0, 0, 0"))
  (if (Variables|Default|GetNeedsTrigger?)
    (Development|PrintString "NEEDS TO ACTIVATE TRIGGER")
    (else
      (CallFunction|OpenClose))))

(fn ConstructionScript
  (|CallParentFunction))