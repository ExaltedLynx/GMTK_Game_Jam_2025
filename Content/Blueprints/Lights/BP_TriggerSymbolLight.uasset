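; BP_TriggerSymbolLight is a symbol light actor with a text label and a cube that can glow.
; The construction script starts the cube unlit by zeroing its Emissive Strength material parameter.
; ToggleEmissionLight switches that parameter between EmissiveLightValue and zero, while SetSymbolText sets the displayed letter.
; Its event graph is empty, so it has no trigger or tick logic of its own.
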(event EventBeginPlay)

(event Collision|EventActorBeginOverlap
  (params (OtherActor :type Actor%20Object%20Reference)))

(event EventTick
  (params (DeltaSeconds :type Float%20%28single-precision%29)))

(fn ConstructionScript
  (Rendering|Material|SetScalarParameterValueonMaterials (Variables|Default|GetCube) "Emissive Strength" 0.0))

(fn SetSymbolText
  (params (SymbolLetter :type Text))
  (Rendering|Components|TextRender|SetText (Variables|Default|GetSymbolText) SymbolLetter))

(fn ToggleEmissionLight
  (params (toggle :type Boolean))
  (bind _cube (Variables|Default|GetCube))
  (if toggle
    (Rendering|Material|SetScalarParameterValueonMaterials _cube "Emissive Strength" (Variables|Default|GetEmissiveLightValue))
    (else
      (Rendering|Material|SetScalarParameterValueonMaterials _cube "Emissive Strength" 0.0))))