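; BP_ItemBase is a base item actor that the player picks up into the inventory.
; On BeginPlay it looks up its ItemName row in the DT_Items data table and caches it as ItemData.
; HandleInteract passes ItemData to TryAddItem on player 0's BP_InventoryComponent and destroys the actor on success.
; A missing row or failed add only prints a debug string.
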(event EventBeginPlay
  (CallFunction|CreateItemfromData))

(event EventHandleInteract
  (params (Interactor :type BP%20First%20Person%20Character%20Object%20Reference) (PrimitiveComp :type Primitive%20Component%20Object%20Reference) (InteractedActor :type Actor%20Object%20Reference) (LocationHit :type Vector :default "0, 0, 0"))
  (bind _success_ (Default|TryAddItem (Actor|GetComponentbyClass (Game|GetPlayerCharacter 0) "/Game/Blueprints/Inventory/BP_InventoryComponent.BP_InventoryComponent_C") (Variables|Default|GetItemData)))
  (if _success_
    (Actor|DestroyActor)
    (else
      (Development|PrintString "Add ITEM Unsuccesful"))))

(fn ConstructionScript)

(fn CreateItemfromData
  (bind _returnvalue (Utilities|GetDataTableRow "/Game/Blueprints/Inventory/Data/DT_Items.DT_Items" (Variables|Default|GetItemName))
    (:then
      (Variables|Default|SetItemData _returnvalue))
    (:RowNotFound
      (Development|PrintString "ITEM NAME NOT FOUND"))))